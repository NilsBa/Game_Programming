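; Player-controlled camera pawn that moves along its forward and right vectors, yaws and zooms from input axes.
; ZoomCamera clamps a target spring arm length and interpolates toward it, easing arm pitch between low and high angles around half of maximum zoom.
; Holding Left Shift switches movement and rotation to their high speeds.
; The left mouse button calls an empty LeftMouseButton function.
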(event `self.ReceiveBeginPlay`
  (bind _output_get (set `SpringArmComponent.TargetArmLength` (/ (`self.MaximumZoomLevel`) 2.0) (`self.SpringArm`)))
  (set `self.NewTargetArmLength` _output_get)
  (set `self.PitchTreshhold` (/ (`self.MaximumZoomLevel`) 2.0))
  (set `self.MovementSpeed` (`self.LowMovementSpeed`))
  (set `self.RotateSpeed` (`self.LowRotateSpeed`)))

(event `InputAxis|MoveForward`
  (params (AxisValue :type "Float (single-precision)"))
  (`self.MoveForward` AxisValue))

(event `InputAxis|MoveRight`
  (params (AxisValue :type "Float (single-precision)"))
  (`self.MoveRight` AxisValue))

(event `InputAxis|RotateCamera`
  (params (AxisValue :type "Float (single-precision)"))
  (`self.RotateCamera` AxisValue))

(event `InputAxis|ZoomCamera`
  (params (AxisValue :type "Float (single-precision)"))
  (`self.ZoomCamera` AxisValue))

(event `InputAction|LeftMouseButton`
  (params (Key :type "Key Structure"))
  (:`Pressed`
    (`self.LeftMouseButton`)))

(event `Key|LeftShift`
  (params (Key :type "Key Structure"))
  (:`Pressed`
    (`self.SpeedUpCamera`))
  (:`Released`
    (`self.SlowDownCamera`)))

(fn `LeftMouseButton`)

(fn `MoveForward`
  (params (AxisValue :type "Float (double-precision)"))
  (`self.AddMovementInput` (`self.GetActorForwardVector`) (* AxisValue (`self.MovementSpeed`))))

(fn `MoveRight`
  (params (AxisValue :type "Float (double-precision)"))
  (`self.AddMovementInput` (`self.GetActorRightVector`) (* AxisValue (`self.MovementSpeed`))))

(fn `RotateCamera`
  (params (AxisValue :type "Float (double-precision)"))
  (`self.K2_SetActorRotation` (`KismetMathLibrary.MakeRotator` (.roll (`self.K2_GetActorRotation`)) (.pitch (`self.K2_GetActorRotation`)) (+ (* AxisValue (`self.RotateSpeed`)) (.yaw (`self.K2_GetActorRotation`))))))

(fn `SlowDownCamera`
  (set `self.MovementSpeed` (`self.LowMovementSpeed`))
  (set `self.RotateSpeed` (`self.LowRotateSpeed`)))

(fn `SpeedUpCamera`
  (set `self.MovementSpeed` (`self.HighMovementSpeed`))
  (set `self.RotateSpeed` (`self.HighRotateSpeed`)))

(fn `UserConstructionScript`)

(fn `ZoomCamera`
  (params (AxisValue :type "Float (double-precision)"))
  (bind _springarm (`self.SpringArm`))
  (bind _output_get (set `self.NewTargetArmLength` (`KismetMathLibrary.FClamp` (+ (* AxisValue (`self.ZoomSpeed`)) (`self.NewTargetArmLength`)) (`self.MinimumZoomLevel`) (`self.MaximumZoomLevel`))))
  (set `SpringArmComponent.TargetArmLength` (`KismetMathLibrary.FInterpTo` (`SpringArmComponent.TargetArmLength` _springarm) _output_get (`GameplayStatics.GetWorldDeltaSeconds`) 15.0) _springarm)
  (if (< (`self.NewTargetArmLength`) (`self.PitchTreshhold`))
    (`SceneComponent.K2_SetRelativeRotation` (`self.SpringArm`) (`KismetMathLibrary.MakeRotator` 0.0 (`KismetMathLibrary.FInterpTo` (.pitch (.rotation (`SceneComponent.GetRelativeTransform` (`self.SpringArm`)))) (`self.CamLowPitch`) (`GameplayStatics.GetWorldDeltaSeconds`) (`self.ZoomInterpSpeed`))) false false)
    (else
      (`SceneComponent.K2_SetRelativeRotation` (`self.SpringArm`) (`KismetMathLibrary.MakeRotator` 0.0 (`KismetMathLibrary.FInterpTo` (.pitch (.rotation (`SceneComponent.GetRelativeTransform` (`self.SpringArm`)))) (`self.CamHighPitch`) (`GameplayStatics.GetWorldDeltaSeconds`) (`self.ZoomInterpSpeed`))) false false))))