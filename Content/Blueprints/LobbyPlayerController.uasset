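; Lobby player controller that owns a player's lobby UI while waiting in a session.
; AddLobbyWB creates W_Lobby with the server's name, map, mode and slots, shows the mouse cursor, and stores the widget for player list and count updates.
; LoadingScreen swaps the lobby widget for W_LoadingScreen.
; Kick opens the Menu level, then destroys the session.
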(event `ClearPlayerList`
  ;[1 1 1] Clear player list
  (`/Game/MainMenu/w_Lobby.ClearPlayerList` (`self.LobbyWidget`)))

(event `Kick`
  ;[1 1 1] kick player
  (`GameplayStatics.OpenLevel` "Menu")
  (`DestroySessionCallbackProxy.DestroySession` self))

(event `AddPlayer`
  (params (Player :type Text) (PlayerIndex :type Integer))
  ;[1 1 1] Add player to list
  (`/Game/MainMenu/w_Lobby.AddPlayerToList` (`self.LobbyWidget`) Player PlayerIndex))

(event `UpdateNumberOfPlayers`
  (params (currentPlayers :type Integer))
  ;[1 1 1] Update Player-Number
  (set `/Game/MainMenu/w_Lobby.currentPlayers` currentPlayers (`self.LobbyWidget`)))

(event `AddLobbyWB`
  (params (ServerName :type String) (ServerMap :type String) (ServerMode :type String) (ServerSlots :type Integer))
  ;[1 1 1] Create Lobby Widget
  (set `self.bShowMouseCursor` true)
  (bind _returnvalue (`|CreateWidget` "/Game/MainMenu/w_Lobby.w_Lobby_C" null (`KismetTextLibrary.Conv_StringToText` ServerName) (`KismetTextLibrary.Conv_StringToText` ServerMap) (`KismetTextLibrary.Conv_StringToText` ServerMode) ServerSlots))
  (bind _output_get (set `self.LobbyWidget` _returnvalue))
  (`UserWidget.AddToViewport` _output_get 1))

(event `LoadingScreen`
  ;[1 1 1] Loading Screen
  (`Widget.RemoveFromParent` (`self.LobbyWidget`))
  (bind _returnvalue (`|CreateWidget` "/Game/MainMenu/W_LoadingScreen.W_LoadingScreen_C" self))
  (`UserWidget.AddToViewport` _returnvalue 0))

(fn `UserConstructionScript`)