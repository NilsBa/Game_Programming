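; In-game GameMode for a two-team unit and tower game that sets up each match and handles spawning.
; On BeginPlay it picks base transforms by level name, then after a short delay spawns a BP_Tower3 base for each team.
; ChoosePlayerStart gives the first controller the first PlayerStart and steps an index for the others.
; It also spawns units from rows, places towers by cloning a unit's class and row, and announces tower destruction through a dispatcher.
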(event `SpawnUnit`
  (params (SpawnTransfrom :type "Transform Structure") (UnitRow :type "DataTableRowHandle Structure"))
  (`|SpawnActorFromClass` "/Game/Blueprint/Unit/BP_Unit.BP_Unit_C" SpawnTransfrom "Undefined" "OverrideRootScale" null UnitRow null))

(event `self.ReceiveBeginPlay`
  (`|ExecutionSequence`
    (:`then_0`
      (bind _returnvalue (`GameplayStatics.GetCurrentLevelName` true))
      (if (`KismetStringLibrary.EqualEqual_StrStr` _returnvalue "Map1")
        (set `self.Base1Transform` (`KismetMathLibrary.MakeTransform` (0.0 -5650.0 100.0)))
        (set `self.Base2Transform` (`KismetMathLibrary.MakeTransform` (0.0 5750.0 100.0) (struct :`Yaw` 180.0)))
        (else
          (set `self.Base1Transform` (`KismetMathLibrary.MakeTransform` (0.0 -10450.0 0.0) (struct)))
          (set `self.Base2Transform` (`KismetMathLibrary.MakeTransform` (0.0 950.0 0.0) (struct :`Yaw` 180.0))))))
    (:`then_1`
      (`KismetSystemLibrary.Delay` 0.1)
      (`self.SpawnBases`))))

(event `SpawnBases`
  (bind _returnvalue (`|SpawnActorFromClass` "/Game/Blueprint/Unit/BP_Tower3.BP_Tower3_C" (`self.Base1Transform`) "Undefined" "OverrideRootScale" null (struct) null))
  (set `/Game/Blueprint/Unit/BP_Unit.Team` 0 _returnvalue)
  (bind _returnvalue_2 (`|SpawnActorFromClass` "/Game/Blueprint/Unit/BP_Tower3.BP_Tower3_C" (`self.Base2Transform`) "Undefined" "OverrideRootScale" null (struct) null))
  (set `/Game/Blueprint/Unit/BP_Unit.Team` 1 _returnvalue_2))

(fn `ChoosePlayerStart`
  (params (Player :type "Controller Object Reference"))
  (returns (ReturnValue :type "Actor Object Reference"))
  (locals (CurrentPlayerStart :type "PlayerStart Object Reference"))
  (bind _playerstartcount (`self.PlayerStartCount`))
  (if (== Player (`GameplayStatics.GetPlayerController` 0))
    (bind _outactors (`GameplayStatics.GetAllActorsOfClass` "/Script/Engine.PlayerStart"))
    (set `self.PlayerStart` _outactors)
    (set `local.CurrentPlayerStart` (`|GetArrayItem` (`self.PlayerStart`)))
    (set `self.PlayerStartCount` 0)
    (else
      (set `self.PlayerStartCount` (+ 1 _playerstartcount))
      (set `local.CurrentPlayerStart` (`|GetArrayItem` (`self.PlayerStart`) _playerstartcount))))
  (return (`local.CurrentPlayerStart`)))

(fn `DestroyTower`
  (params (BPUnit :type "/Game/Blueprint/Unit/BP_Unit Object Reference"))
  (set `self.TowerToDestroyRef` BPUnit)
  (`self.DestroyTowerDispatcher`))

(fn `GetTowerToDestroy`
  (returns (TowerRef :type "/Game/Blueprint/Unit/BP_Unit Object Reference"))
  (return (`self.TowerToDestroyRef`)))

(fn `SpawnTower`
  (params (TowerPlaced :type Boolean) (SpawnTransform :type "Transform Structure") (BPUnit :type "/Game/Blueprint/Unit/BP_Unit Object Reference"))
  (returns (Placed :type Boolean) (TowerRef :type "/Game/Blueprint/Unit/BP_Unit Object Reference") (ChangeRef :type Boolean))
  (if TowerPlaced
    (return true null false)
    (elif (`KismetSystemLibrary.IsValid` BPUnit)
      (bind _returnvalue (`|SpawnActorFromClass` (`GameplayStatics.GetObjectClass` BPUnit) SpawnTransform "Undefined" "OverrideRootScale" null (`/Game/Blueprint/Unit/BP_Unit.UnitRow` BPUnit) null))
      (return true _returnvalue true)
      (else
        (return false null false)))))

(fn `UserConstructionScript`
  (`parent.UserConstructionScript`))