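; BP_Tower2 is a tower unit that turns toward its target every tick and attacks with paired homing missiles.
; The multicast attack event fires from two scene points half a second apart, spawning short-lived missiles with the particle template from the unit data row.
; On death it spawns a temporary Tower2Mesh_DMBlue actor at the body's transform and calls DestroyTower on the game mode.
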(event `self.ReceiveTick`
  (params (DeltaSeconds :type "Float (single-precision)"))
  (`parent.ReceiveTick` DeltaSeconds)
  (`self.RotateToTarget`))

(event `self.Multicast_TriggerAttack`
  (`self.Shoot1`)
  (`KismetSystemLibrary.Delay` 0.5)
  (`self.Shoot2`))

(fn `OnDeath`
  (`parent.OnDeath`)
  (bind _returnvalue (`|SpawnActorFromClass` "/Game/Towers/Tower2Mesh_DMBlue.Tower2Mesh_DMBlue_C" (`SceneComponent.K2_GetComponentToWorld` (`self.Body2`)) "AdjustIfPossibleButAlwaysSpawn" "OverrideRootScale" null null))
  (`self.SetLifeSpan` _returnvalue 2.0)
  (bind _asbp_ingame_mode (cast `/Game/Blueprint/GameSystem/BP_IngameMode` (`GameplayStatics.GetGameMode`)))
  (`/Game/Blueprint/GameSystem/BP_IngameMode.DestroyTower` _asbp_ingame_mode self))

(fn `Shoot1`
  (bind _attacktarget (`self.AttackTarget`))
  (bind _returnvalue (`|SpawnActorFromClass` "/Game/Blueprint/Unit/Utils/HomingMissile.HomingMissile_C" (`KismetMathLibrary.MakeTransform` (`SceneComponent.K2_GetComponentLocation` (`self.Scene1`)) (`KismetMathLibrary.FindLookAtRotation` (`self.K2_GetActorLocation`) (`self.K2_GetActorLocation` _attacktarget)) (0.5 0.5 0.5)) "Undefined" "OverrideRootScale" null self))
  (`/Engine/EditorBlueprintResources/StandardMacros.IsValid` _returnvalue
    (:`Is Valid`
      (`ParticleSystemComponent.SetTemplate` (`/Game/Blueprint/Unit/Utils/HomingMissile.ParticleSystem` _returnvalue) (`.Projectile_65_FC29291B45ED7828020C34B0C003EADA` (break `/Game/Blueprint/Unit/Utils/FUnit` (`self.UnitDataRow`))))
      (set `/Game/Blueprint/Unit/Utils/HomingMissile.HomingTarget` _attacktarget _returnvalue)
      (`self.SetLifeSpan` _returnvalue 0.5))))

(fn `Shoot2`
  (bind _attacktarget (`self.AttackTarget`))
  (`/Engine/EditorBlueprintResources/StandardMacros.IsValid` _attacktarget
    (:`Is Valid`
      (bind _returnvalue (`|SpawnActorFromClass` "/Game/Blueprint/Unit/Utils/HomingMissile.HomingMissile_C" (`KismetMathLibrary.MakeTransform` (`SceneComponent.K2_GetComponentLocation` (`self.Scene`)) (`KismetMathLibrary.FindLookAtRotation` (`self.K2_GetActorLocation`) (`self.K2_GetActorLocation` _attacktarget)) (0.5 0.5 0.5)) "Undefined" "OverrideRootScale" null self))
      (`/Engine/EditorBlueprintResources/StandardMacros.IsValid` _returnvalue
        (:`Is Valid`
          (`ParticleSystemComponent.SetTemplate` (`/Game/Blueprint/Unit/Utils/HomingMissile.ParticleSystem` _returnvalue) (`.Projectile_65_FC29291B45ED7828020C34B0C003EADA` (break `/Game/Blueprint/Unit/Utils/FUnit` (`self.UnitDataRow`))))
          (set `/Game/Blueprint/Unit/Utils/HomingMissile.HomingTarget` _attacktarget _returnvalue)
          (`self.SetLifeSpan` _returnvalue 0.5))))))

(fn `UserConstructionScript`
  (`parent.UserConstructionScript`))