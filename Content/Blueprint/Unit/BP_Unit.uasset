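; Base combat unit for a square-based two-team battle game, configured from a DT_Units row (mesh, capsule, stats, role flags) and team-tinted.
; It snaps onto BP_Square tiles, supports drag and focus outline, and drives AI through blackboard keys.
; Attacks deal direct damage or fire homing missiles resolved on overlap, with healer and siege-versus-priority rules.
; CurrentHealth's RepNotify broadcasts changes and triggers death, which reports to both player controllers.
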(event `self.ReceiveBeginPlay`
  (`self.ExtractDataFromRow`)
  (`self.FindSquare`)
  (`self.SetTeamColor`))

(event `self.ReceiveActorBeginOverlap`
  (params (OtherActor :type "Actor Object Reference"))
  (bind _ashoming_missile (cast `/Game/Blueprint/Unit/Utils/HomingMissile` OtherActor))
  (bind _asbp_unit (cast `/Game/Blueprint/Unit/BP_Unit` (`self.GetInstigator` _ashoming_missile)))
  (if (== (`/Game/Blueprint/Unit/BP_Unit.AttackTarget` _asbp_unit) self)
    (bind ((`Damage_24_A523A1B7445923E09C59FFB3EA471650` _damage) (`isSiege_41_6C47FDDF4E8DDA3D50C6B8AA8CB87882` _issiege) (`isHealer_42_4CF1FCBF4D59B5994F75FCA7AC022656` _ishealer) (`isBase_78_64882331482F417B900EE0A2B645FB56` _isbase) (`HitEffect_69_DE6BB3F94E2F71A1057E4AB20816A6B2` _hiteffect)) (break `/Game/Blueprint/Unit/Utils/FUnit` (`/Game/Blueprint/Unit/BP_Unit.UnitDataRow` _asbp_unit)))
    (if (and _issiege (`self.bHasPriority`))
      (bind _returnvalue (`self.K2_GetActorLocation` _ashoming_missile))
      (`GameplayStatics.SpawnEmitterAtLocation` _hiteffect _returnvalue (struct) (4.0 4.0 4.0))
      (else
        (`GameplayStatics.SpawnEmitterAtLocation` _hiteffect _returnvalue)))
    (if (and (== (`/Game/Blueprint/Unit/BP_Unit.Team` _asbp_unit) (`self.Team`)) _ishealer)
      (`self.OnHeal` _damage)
      (else
        (`self.OnTakeDamage` _damage _asbp_unit)))
    (`self.K2_DestroyActor` _ashoming_missile)))

(event `self.ReceiveTick`
  (params (DeltaSeconds :type "Float (single-precision)"))
  (`self.RefreshTarget`)
  (if (not (`self.bHasPriority`))
    (`self.RotateTowardsMovement`)
    (`self.RotateToTarget`)))

(event `Multicast_TriggerAttack`
  (`|PlayMontage` (`self.SkeletalMesh`) (`.AttackMontage_17_6420CB4746EB8D153ECF2A8D084A6297` (break `/Game/Blueprint/Unit/Utils/FUnit` (`self.UnitDataRow`)))
    (:`then`
      (if (`self.bIsRanged`)
        _))))

(event `TriggerAttack`
  (bind _attacktarget (`self.AttackTarget`))
  (bind (_name _skeletalmesh _animinstance _attackmontage _health _damage _attackspeed _isranged _haspriority _issiege _ishealer _isbase _materials _materialparameters _projectile _hiteffect _capsulehalfheight _capsuleradius _sound) (break `/Game/Blueprint/Unit/Utils/FUnit` (`self.UnitDataRow`)))
  (`/Engine/EditorBlueprintResources/StandardMacros.IsValid` (`self.AttackTarget`)
    (:`Is Valid`
      (`|ExecutionSequence`
        (:`then_0`
          (`self.Multicast_TriggerAttack`))
        (:`then_1`
          (`KismetSystemLibrary.Delay` 0.3)
          (`GameplayStatics.SpawnSound2D` _sound 1.0 1.0 0.0 null)
          (if _isranged
            (`self.Shoot` null)
            (else
              (`/Engine/EditorBlueprintResources/StandardMacros.IsValid` _attacktarget
                (:`Is Valid`
                  (`self.OnTakeDamage` _attacktarget _damage self _sound))))))))))

(event `Shoot`
  (params (Sounds :type "SoundCue Object Reference"))
  (bind _attacktarget (`self.AttackTarget`))
  (`/Engine/EditorBlueprintResources/StandardMacros.IsValid` _attacktarget
    (:`Is Valid`
      (bind _returnvalue (`|SpawnActorFromClass` "/Game/Blueprint/Unit/Utils/HomingMissile.HomingMissile_C" (`KismetMathLibrary.MakeTransform` (`SceneComponent.K2_GetComponentLocation` (`self.Scene`)) (`KismetMathLibrary.FindLookAtRotation` (`self.K2_GetActorLocation`) (`self.K2_GetActorLocation` _attacktarget)) (0.5 0.5 0.5)) "Undefined" "OverrideRootScale" null self))
      (`/Engine/EditorBlueprintResources/StandardMacros.IsValid` _returnvalue
        (:`Is Valid`
          (`ParticleSystemComponent.SetTemplate` (`/Game/Blueprint/Unit/Utils/HomingMissile.ParticleSystem` _returnvalue) (`.Projectile_65_FC29291B45ED7828020C34B0C003EADA` (break `/Game/Blueprint/Unit/Utils/FUnit` (`self.UnitDataRow`))))
          (set `/Game/Blueprint/Unit/Utils/HomingMissile.HomingTarget` _attacktarget _returnvalue)
          (`self.SetLifeSpan` _returnvalue 0.5))))))

(fn `ExtractDataFromRow`
  (bind _skeletalmesh (`self.SkeletalMesh`))
  (bind _returnvalue (`AIBlueprintHelperLibrary.GetBlackboard` (`self.GetController`)))
  (bind _returnvalue_2 (`|GetDataTableRow` "/Game/Data/DT_Units.DT_Units" (`.RowName` (break `DataTableRowHandle` (`self.UnitRow`))))
    (:`then`
      (bind _output_get (set `self.UnitDataRow` _returnvalue_2))
      (bind (_name _skeletalmesh_2 _animinstance _attackmontage _health _damage _attackspeed _isranged _haspriority _issiege _ishealer _isbase _materials _materialparameters _projectile _hiteffect _capsulehalfheight _capsuleradius) (break `/Game/Blueprint/Unit/Utils/FUnit` _output_get))
      (`SkinnedMeshComponent.SetSkinnedAssetAndUpdate` _skeletalmesh _skeletalmesh_2 true)
      (`SkeletalMeshComponent.SetAnimInstanceClass` _skeletalmesh _animinstance)
      (bind _output_get_2 (set `self.bIsRanged` _isranged))
      (bind _output_get_3 (set `self.bHasPriority` _haspriority))
      (set `self.bIsSiege` _issiege)
      (set `self.bIsHealer` _ishealer)
      (set `self.bIsBase` _isbase)
      (`CapsuleComponent.SetCapsuleSize` (`self.Capsule`) _capsuleradius _capsulehalfheight true)
      (`/Engine/EditorBlueprintResources/StandardMacros.IsValid` _returnvalue
        (:`Is Valid`
          (`BlackboardComponent.SetValueAsBool` _returnvalue "isRanged" _output_get_2)
          (`BlackboardComponent.SetValueAsBool` _returnvalue "hasPriority" _output_get_3)
          (`BlackboardComponent.SetValueAsFloat` _returnvalue "AttackSpeed" _attackspeed))
        (:`Is Not Valid`
          _))
      (bind _output_get_4 (set `self.MaxHealth` _health))
      (set `self.CurrentHealth` _output_get_4))))

(fn `FindSquare`
  (bind _returnvalue (`self.K2_GetActorLocation`))
  (bind _initialsquare (`self.InitialSquare`))
  (`/Engine/EditorBlueprintResources/StandardMacros.IsValid` _initialsquare
    (:`Is Valid`
      (set `/Game/Blueprint/Level/BP_Square.HostedUnit` null _initialsquare))
    (:`Is Not Valid`
      _))
  (bind _outhits (`KismetSystemLibrary.SphereTraceMulti` _returnvalue (+ _returnvalue (0.0 0.0 1.0)) 5.0 "TraceTypeQuery4"))
  (for _array_element _outhits
    (bind (_bblockinghit _binitialoverlap _time _distance _location _impactpoint _normal _impactnormal _physmat _hitactor) (`GameplayStatics.BreakHitResult` _array_element))
    (if (== (`GameplayStatics.GetObjectClass` _hitactor) "/Game/Blueprint/Level/BP_Square.BP_Square_C")
      (bind _asbp_square (cast `/Game/Blueprint/Level/BP_Square` _hitactor))
      (set `/Game/Blueprint/Level/BP_Square.HostedUnit` self _asbp_square)
      (bind _returnvalue_2 (`GameplayStatics.GetCurrentLevelName` true))
      (if (`KismetStringLibrary.EqualEqual_StrStr` _returnvalue_2 "Map1")
        (bind _x (.x (`self.K2_GetActorLocation` _asbp_square)))
        (bind _y (.y (`self.K2_GetActorLocation` _asbp_square)))
        (bind _returnvalue_3 (+ (.z (`self.K2_GetActorLocation` _asbp_square)) (`CapsuleComponent.GetScaledCapsuleHalfHeight` (`self.Capsule`))))
        (`self.K2_SetActorLocation` (`KismetMathLibrary.MakeVector` _x _y _returnvalue_3))
        (set `self.InitialSquare` _asbp_square)
        (else
          (`self.K2_SetActorLocation` (`KismetMathLibrary.MakeVector` _x _y (+ _returnvalue_3 100.0)))
          (set `self.InitialSquare` null))))))

(fn `GetGameStateRef`
  (returns (ReturnValue :type "/Game/Blueprint/GameSystem/BP_GameState Object Reference"))
  (`/Engine/EditorBlueprintResources/StandardMacros.IsValid` (`self.GameStateRef`)
    (:`Is Valid`
      _)
    (:`Is Not Valid`
      (bind _asbp_game_state (cast `/Game/Blueprint/GameSystem/BP_GameState` (`GameplayStatics.GetGameState`)))
      (set `self.GameStateRef` _asbp_game_state)))
  (return (`self.GameStateRef`)))

(fn `OnDeath`
  (`self.Dispatch_OnDeath` self)
  (`self.SetAIState` "NewEnumerator3")
  (`SceneComponent.SetVisibility` (`self.Capsule`) false true)
  (`self.SetActorEnableCollision` false)
  (`|ExecutionSequence`
    (:`then_0`
      (bind _asbp_ingame_player_controller (cast `/Game/Blueprint/Player/BP_IngamePlayerController` (`GameplayStatics.GetPlayerController` 0)))
      (`/Game/Blueprint/Player/BP_IngamePlayerController.AddUnitDeath` _asbp_ingame_player_controller (`self.Team`)))
    (:`then_1`
      (bind _asbp_ingame_player_controller_2 (cast `/Game/Blueprint/Player/BP_IngamePlayerController` (`GameplayStatics.GetPlayerController` 1)))
      (`/Game/Blueprint/Player/BP_IngamePlayerController.AddUnitDeath` _asbp_ingame_player_controller_2 (`self.Team`)))))

(fn `OnHeal`
  (params (Amount :type "Float (double-precision)"))
  (set `self.CurrentHealth` (`KismetMathLibrary.FClamp` (+ (`self.CurrentHealth`) Amount) 0.0 (`self.MaxHealth`))))

(fn `OnRep_CurrentHealth`
  (`self.Dispatch_OnHealthModify` (`self.CurrentHealth`))
  (if (== (`self.CurrentHealth`) 0.0)
    (`self.OnDeath`)))

(fn `OnTakeDamage`
  (params (Amount :type "Float (double-precision)") (DamageDealer :type "/Game/Blueprint/Unit/BP_Unit Object Reference") (Sounds :type "SoundCue Object Reference"))
  (if (and (`/Game/Blueprint/Unit/BP_Unit.bIsSiege` DamageDealer) (`self.bHasPriority`))
    (set `self.CurrentHealth` (`KismetMathLibrary.FClamp` (- (`self.CurrentHealth`) (* Amount 2.0)) 0.0 (`self.MaxHealth`)))
    (else
      (set `self.CurrentHealth` (`KismetMathLibrary.FClamp` (- (`self.CurrentHealth`) Amount) 0.0 (`self.MaxHealth`))))))

(fn `RefreshTarget`
  (bind _attacktarget (`self.AttackTarget`))
  (`/Engine/EditorBlueprintResources/StandardMacros.IsValid` _attacktarget
    (:`Is Valid`
      (if (or (`|EnumEquality` (`/Game/Blueprint/Unit/BP_Unit.AIState` _attacktarget) "NewEnumerator3") (and (`self.bIsHealer`) (== (`/Game/Blueprint/Unit/BP_Unit.CurrentHealth` _attacktarget) (`/Game/Blueprint/Unit/BP_Unit.MaxHealth` _attacktarget)) (== (`/Game/Blueprint/Unit/BP_Unit.Team` _attacktarget) (`self.Team`))))
        (set `self.AttackTarget` null)))))

(fn `RotateToTarget`
  (bind _attacktarget (`self.AttackTarget`))
  (bind _returnvalue (`KismetMathLibrary.MakeRotator` 0.0 0.0 (.yaw (`self.K2_GetActorRotation`))))
  (bind _returnvalue_2 (`KismetMathLibrary.MakeRotator` 0.0 0.0 (- (.yaw (`KismetMathLibrary.FindLookAtRotation` (`self.K2_GetActorLocation`) (`self.K2_GetActorLocation` _attacktarget))) 90.0)))
  (`/Engine/EditorBlueprintResources/StandardMacros.IsValid` _attacktarget
    (:`Is Valid`
      (if (`self.bShouldRotate`)
        (`self.K2_SetActorRotation` (`KismetMathLibrary.RInterpTo` _returnvalue _returnvalue_2 (`GameplayStatics.GetWorldDeltaSeconds`) (`self.RotationSpeed`)))
        (if (== _returnvalue _returnvalue_2 :`ErrorTolerance` 1.0)
          (set `self.bShouldRotate` false))))))

(fn `RotateTowardsMovement`
  (bind _returnvalue (`self.GetVelocity`))
  (bind _returnvalue_2 (`self.K2_GetActorLocation`))
  (if (`self.bShouldRotate`)
    _
    (elif (> (`KismetMathLibrary.VSize` _returnvalue) 0.0)
      (`self.K2_SetActorRotation` (`KismetMathLibrary.RInterpTo` (`self.K2_GetActorRotation`) (`KismetMathLibrary.MakeRotator` (.roll (`KismetMathLibrary.FindLookAtRotation` _returnvalue_2 (+ (* _returnvalue 100.0) _returnvalue_2))) (.pitch (`KismetMathLibrary.FindLookAtRotation` _returnvalue_2 (+ (* _returnvalue 100.0) _returnvalue_2))) (- (.yaw (`KismetMathLibrary.FindLookAtRotation` _returnvalue_2 (+ (* _returnvalue 100.0) _returnvalue_2))) 90.0)) (`GameplayStatics.GetWorldDeltaSeconds`) (`self.RotationSpeed`))))))

(fn `SetAIState`
  (params (Enum :type "/Game/Blueprint/AI/Utils/EUnitState Enum" :default "NewEnumerator0"))
  (`/Engine/EditorBlueprintResources/ActorMacros.Switch Has Authority`
    (:`Authority`
      (bind _output_get (set `self.AIState` Enum))
      (`BlackboardComponent.SetValueAsEnum` (`AIBlueprintHelperLibrary.GetBlackboard` (`self.GetController`)) "State" _output_get))))

(fn `SetAttackedTarget`
  (returns (ChosenTarget :type "/Game/Blueprint/Unit/BP_Unit Object Reference"))
  (bind _returnvalue (`/Game/Blueprint/Level/BP_Battlefield.GetClosestEnemyUnit` (`self.Battlefield`) self))
  (`/Engine/EditorBlueprintResources/ActorMacros.Switch Has Authority`
    (:`Authority`
      (`/Engine/EditorBlueprintResources/StandardMacros.IsValid` _returnvalue
        (:`Is Valid`
          (bind _output_get (set `self.AttackTarget` _returnvalue)))
        (:`Is Not Valid`
          _))
      (return _output_get))))

(fn `SetDragState`
  (params (bEnabled :type Boolean))
  (bind _skeletalmesh (`self.SkeletalMesh`))
  (`self.SetMeshRelativeZState` bEnabled)
  (if bEnabled
    (`SceneComponent.K2_SetRelativeRotation` _skeletalmesh (struct :`Roll` 25.0) false false)
    (else
      (`SceneComponent.K2_SetRelativeRotation` :`self` _skeletalmesh))))

(fn `SetFocused`
  (params (bFocused :type Boolean))
  (bind _skeletalmesh (`self.SkeletalMesh`))
  (if bFocused
    (`PrimitiveComponent.SetRenderCustomDepth` _skeletalmesh true)
    (`PrimitiveComponent.SetCustomDepthStencilValue` _skeletalmesh 250)
    (else
      (`PrimitiveComponent.SetRenderCustomDepth` _skeletalmesh false))))

(fn `SetMeshRelativeZState`
  (params (bDragged :type Boolean))
  (bind _skeletalmesh (`self.SkeletalMesh`))
  (bind _returnvalue (`SkeletalMeshComponent.GetAnimInstance` _skeletalmesh))
  (if bDragged
    (`SceneComponent.K2_SetRelativeLocation` _skeletalmesh (`KismetMathLibrary.MakeVector` 0.0 0.0 100.0) false false)
    (message `/Game/Blueprint/Unit/Utils/BPI_AnimCommunication.SetDraggedAnimState` _returnvalue true)
    (else
      (`SceneComponent.K2_SetRelativeLocation` (`self.SkeletalMesh`) (`KismetMathLibrary.MakeVector` 0.0 0.0 -50.0) false false)
      (message `/Game/Blueprint/Unit/Utils/BPI_AnimCommunication.SetDraggedAnimState` _returnvalue false))))

(fn `SetTeamColor`
  (bind (_name _skeletalmesh _animinstance _attackmontage _health _damage _attackspeed _isranged _haspriority _issiege _ishealer _isbase _materials _materialparameters) (break `/Game/Blueprint/Unit/Utils/FUnit` (`self.UnitDataRow`)))
  (for (_ _array_index) _materials
    (bind _returnvalue (`PrimitiveComponent.CreateDynamicMaterialInstance` (`self.SkeletalMesh`) _array_index null "None"))
    (for _array_element _materialparameters
      (`MaterialInstanceDynamic.SetVectorParameterValue` _returnvalue _array_element (`/Game/Blueprint/GameSystem/BP_GameState.GetTeamColor` (`self.GetGameStateRef`) (`self.Team`))))))

(fn `StartCombat`
  (if (`|EnumInequality` (`self.AIState`) "NewEnumerator3")
    (`self.SetAIState` "NewEnumerator1")))

(fn `UserConstructionScript`
  (`self.ExtractDataFromRow`)
  (`SceneComponent.K2_SetRelativeLocation` (`self.SkeletalMesh`) (`KismetMathLibrary.MakeVector` 0.0 0.0 (* (`CapsuleComponent.GetScaledCapsuleHalfHeight` (`self.Capsule`)) -1.0)) false false)
  (`self.FindSquare`)
  (set `self.Team` (`KismetMathLibrary.FTrunc` (`KismetMathLibrary.Abs` (/ (.yaw (`self.K2_GetActorRotation`)) 179.0)))))