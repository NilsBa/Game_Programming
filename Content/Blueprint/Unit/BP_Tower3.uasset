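; Tower unit whose death ends the match with its team as the loser and spawns a destructible mesh in its place.
; Its multicast attack fires three homing missiles one second apart from separate scene points, using the projectile effect from the unit data row.
; Damage plays sounds through the team's player controller, adding a custom-depth blink below quarter health.
; FindSquare sphere-traces for a board square, registers as its hosted unit and snaps onto it.
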(event `self.ReceiveTick`
  (params (DeltaSeconds :type "Float (single-precision)"))
  (`parent.ReceiveTick` DeltaSeconds))

(event `self.Multicast_TriggerAttack`
  (`self.Shoot1`)
  (`KismetSystemLibrary.Delay` 1.0)
  (`self.Shoot2`)
  (`KismetSystemLibrary.Delay` 1.0)
  (`self.Shoot3`))

(event `BlinkOnLowHealth`
  (bind _body (`self.Body`))
  (bind _middlebody (`self.MiddleBody`))
  (`PrimitiveComponent.SetRenderCustomDepth` _body true)
  (`PrimitiveComponent.SetCustomDepthStencilValue` _body 249)
  (`PrimitiveComponent.SetRenderCustomDepth` _middlebody true)
  (`PrimitiveComponent.SetCustomDepthStencilValue` _middlebody 249)
  (`KismetSystemLibrary.Delay` 0.5)
  (`PrimitiveComponent.SetRenderCustomDepth` (`self.Body`) false)
  (`PrimitiveComponent.SetRenderCustomDepth` (`self.MiddleBody`) false)
  (`KismetSystemLibrary.Delay` 0.5))

(event `Shoot2`
  (bind _attacktarget (`self.AttackTarget`))
  (`/Engine/EditorBlueprintResources/StandardMacros.IsValid` _attacktarget
    (:`Is Valid`
      (bind _returnvalue (`|SpawnActorFromClass` "/Game/Blueprint/Unit/Utils/HomingMissile.HomingMissile_C" (`KismetMathLibrary.MakeTransform` (`SceneComponent.K2_GetComponentLocation` (`self.Scene1`)) (`KismetMathLibrary.FindLookAtRotation` (`self.K2_GetActorLocation`) (`self.K2_GetActorLocation` _attacktarget))) "Undefined" "OverrideRootScale" null self))
      (`/Engine/EditorBlueprintResources/StandardMacros.IsValid` _returnvalue
        (:`Is Valid`
          (`ParticleSystemComponent.SetTemplate` (`/Game/Blueprint/Unit/Utils/HomingMissile.ParticleSystem` _returnvalue) (`.Projectile_65_FC29291B45ED7828020C34B0C003EADA` (break `/Game/Blueprint/Unit/Utils/FUnit` (`self.UnitDataRow`))))
          (set `/Game/Blueprint/Unit/Utils/HomingMissile.HomingTarget` _attacktarget _returnvalue)
          (`self.SetLifeSpan` _returnvalue 0.5))))))

(event `Shoot3`
  (bind _attacktarget (`self.AttackTarget`))
  (`/Engine/EditorBlueprintResources/StandardMacros.IsValid` _attacktarget
    (:`Is Valid`
      (bind _returnvalue (`|SpawnActorFromClass` "/Game/Blueprint/Unit/Utils/HomingMissile.HomingMissile_C" (`KismetMathLibrary.MakeTransform` (`SceneComponent.K2_GetComponentLocation` (`self.Scene`)) (`KismetMathLibrary.FindLookAtRotation` (`self.K2_GetActorLocation`) (`self.K2_GetActorLocation` _attacktarget))) "Undefined" "OverrideRootScale" null self))
      (`/Engine/EditorBlueprintResources/StandardMacros.IsValid` _returnvalue
        (:`Is Valid`
          (`ParticleSystemComponent.SetTemplate` (`/Game/Blueprint/Unit/Utils/HomingMissile.ParticleSystem` _returnvalue) (`.Projectile_65_FC29291B45ED7828020C34B0C003EADA` (break `/Game/Blueprint/Unit/Utils/FUnit` (`self.UnitDataRow`))))
          (set `/Game/Blueprint/Unit/Utils/HomingMissile.HomingTarget` _attacktarget _returnvalue)
          (`self.SetLifeSpan` _returnvalue 0.5))))))

(event `Shoot1`
  (bind _attacktarget (`self.AttackTarget`))
  (`/Engine/EditorBlueprintResources/StandardMacros.IsValid` _attacktarget
    (:`Is Valid`
      (bind _returnvalue (`|SpawnActorFromClass` "/Game/Blueprint/Unit/Utils/HomingMissile.HomingMissile_C" (`KismetMathLibrary.MakeTransform` (`SceneComponent.K2_GetComponentLocation` (`self.Scene2`)) (`KismetMathLibrary.FindLookAtRotation` (`self.K2_GetActorLocation`) (`self.K2_GetActorLocation` _attacktarget))) "Undefined" "OverrideRootScale" null self))
      (`/Engine/EditorBlueprintResources/StandardMacros.IsValid` _returnvalue
        (:`Is Valid`
          (`ParticleSystemComponent.SetTemplate` (`/Game/Blueprint/Unit/Utils/HomingMissile.ParticleSystem` _returnvalue) (`.Projectile_65_FC29291B45ED7828020C34B0C003EADA` (break `/Game/Blueprint/Unit/Utils/FUnit` (`self.UnitDataRow`))))
          (set `/Game/Blueprint/Unit/Utils/HomingMissile.HomingTarget` _attacktarget _returnvalue)
          (`self.SetLifeSpan` _returnvalue 0.5))))))

(fn `FindSquare`
  (bind _returnvalue (`self.K2_GetActorLocation`))
  (bind _initialsquare (`self.InitialSquare`))
  (`/Engine/EditorBlueprintResources/StandardMacros.IsValid` _initialsquare
    (:`Is Valid`
      (set `/Game/Blueprint/Level/BP_Square.HostedUnit` null _initialsquare))
    (:`Is Not Valid`
      _))
  (bind _outhits (`KismetSystemLibrary.SphereTraceMulti` _returnvalue (+ _returnvalue (0.0 0.0 1.0)) 5.0 "TraceTypeQuery4"))
  (for _array_element _outhits
    (bind (_bblockinghit _binitialoverlap _time _distance _location _impactpoint _normal _impactnormal _physmat _hitactor) (`GameplayStatics.BreakHitResult` _array_element))
    (if (== (`GameplayStatics.GetObjectClass` _hitactor) "/Game/Blueprint/Level/BP_Square.BP_Square_C")
      (bind _asbp_square (cast `/Game/Blueprint/Level/BP_Square` _hitactor))
      (set `/Game/Blueprint/Level/BP_Square.HostedUnit` self _asbp_square)
      (`self.K2_SetActorLocation` (`KismetMathLibrary.MakeVector` (.x (`self.K2_GetActorLocation` _asbp_square)) (.y (`self.K2_GetActorLocation` _asbp_square)) (.z (`self.K2_GetActorLocation` _asbp_square))))
      (set `self.InitialSquare` _asbp_square))))

(fn `OnDeath`
  (bind _team (`self.Team`))
  (`parent.OnDeath`)
  (bind _returnvalue (`|SpawnActorFromClass` "/Game/Towers/Tower3Mesh_DMBlue.Tower3Mesh_DMBlue_C" (`KismetMathLibrary.MakeTransform` (.location (`SceneComponent.K2_GetComponentToWorld` (`self.Body`))) (.rotation (`SceneComponent.K2_GetComponentToWorld` (`self.Body`))) (1.7 1.7 1.7)) "AdjustIfPossibleButAlwaysSpawn" "OverrideRootScale" null null))
  (`self.SetLifeSpan` _returnvalue 10.0)
  (bind _asbp_ingame_player_controller (cast `/Game/Blueprint/Player/BP_IngamePlayerController` (`GameplayStatics.GetPlayerController` _team)))
  (`/Game/Blueprint/Player/BP_IngamePlayerController.EndScreen` _asbp_ingame_player_controller _team (`GameplayStatics.GetPlayerController` _team)))

(fn `OnTakeDamage`
  (params (Amount :type "Float (double-precision)") (DamageDealer :type "/Game/Blueprint/Unit/BP_Unit Object Reference"))
  (`parent.OnTakeDamage` Amount DamageDealer)
  (bind _asbp_ingame_player_controller (cast `/Game/Blueprint/Player/BP_IngamePlayerController` (`GameplayStatics.GetPlayerController` (`self.Team`))))
  (`/Game/Blueprint/Player/BP_IngamePlayerController.PlayDamageSound` _asbp_ingame_player_controller)
  (if (< (`self.CurrentHealth`) (* (`self.MaxHealth`) 0.25))
    (`self.BlinkOnLowHealth`)
    (`/Game/Blueprint/Player/BP_IngamePlayerController.PlayLowHealthSound` _asbp_ingame_player_controller)))

(fn `UserConstructionScript`
  (`parent.UserConstructionScript`))