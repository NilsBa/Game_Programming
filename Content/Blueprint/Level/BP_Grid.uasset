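; Grid actor that lays out a board of BP_Square tiles able to host units.
; The construction script spawns tiles as child actor components across GridSize, spaced by SquareClass's default Size, and stores them in Squares.
; FindUnitsInGrid gathers unique valid hosted units into Units.
; CopyUnits maps each index of a given square array to its hosted unit, including empty squares, as both validity branches add the entry.
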(fn `BuildGrid`
  (bind (_x _y) (`KismetMathLibrary.BreakVector2D` (`self.GridSize`)))
  (bind _size (defaults `Object` (`self.SquareClass`)))
  (for _index (range (+ (`KismetMathLibrary.FTrunc` (- _x 1.0)) 1))
    (for _index_2 (range (+ (`KismetMathLibrary.FTrunc` (- _y 1.0)) 1))
      (bind _returnvalue (`AddComponent|NODE_AddChildActorComponent-0` :`RelativeTransform` (`KismetMathLibrary.MakeTransform` (`KismetMathLibrary.MakeVector` (* _index _size) (* _index_2 _size)))))
      (bind _asbp_square (cast `/Game/Blueprint/Level/BP_Square` (`ChildActorComponent.ChildActor` _returnvalue)))
      (`KismetArrayLibrary.Array_Add` (`self.Squares`) _asbp_square))))

(fn `CopyUnits`
  (params (Squares :type "Array of /Game/Blueprint/Level/BP_Square Object Reference"))
  (returns (UnitsToCopy :type "Map of Integer to /Game/Blueprint/Unit/BP_Unit Object Reference"))
  (bind _unitstocopy (`self.UnitsToCopy`))
  (for (_array_element _array_index) Squares
    (bind _hostedunit (`/Game/Blueprint/Level/BP_Square.HostedUnit` _array_element))
    (`/Engine/EditorBlueprintResources/StandardMacros.IsValid` _hostedunit
      (:`Is Valid`
        (`BlueprintMapLibrary.Map_Add` _unitstocopy _array_index _hostedunit))
      (:`Is Not Valid`
        (`BlueprintMapLibrary.Map_Add` _unitstocopy _array_index _hostedunit))))
  (return (`self.UnitsToCopy`)))

(fn `FindUnitsInGrid`
  (for _array_element (`self.Squares`)
    (bind _hostedunit (`/Game/Blueprint/Level/BP_Square.HostedUnit` _array_element))
    (`/Engine/EditorBlueprintResources/StandardMacros.IsValid` _hostedunit
      (:`Is Valid`
        (`KismetArrayLibrary.Array_AddUnique` (`self.Units`) _hostedunit)))))

(fn `UserConstructionScript`
  (`self.BuildGrid`))