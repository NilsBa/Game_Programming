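; Grid battlefield actor that spawns two teams of units, starts their combat and tracks who is alive.
; StartCombat registers units hosted on squares by team, binding death events that remove them from their team.
; SpawnUnits places BT_Unit-driven AI in centered formations on opposing sides, shifting by tower distance when the area is flagged occupied.
; Helpers check whether a formation area is free and find a unit's closest enemy.
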(fn `FindUnitsInBattlefield`
  (locals (tempUnitArray :type "Array of /Game/Blueprint/Unit/BP_Unit Object Reference"))
  (bind _unitsfromteam (`self.UnitsFromTeam`))
  (for _array_element (`self.Squares`)
    (bind _hostedunit (`/Game/Blueprint/Level/BP_Square.HostedUnit` _array_element))
    (`/Engine/EditorBlueprintResources/StandardMacros.IsValid` _hostedunit
      (:`Is Valid`
        (set `/Game/Blueprint/Unit/BP_Unit.Battlefield` self _hostedunit)
        (bind _team (`/Game/Blueprint/Unit/BP_Unit.Team` _hostedunit))
        (set `local.tempUnitArray` (`.Units_3_D36FB76C40AE2CBD0FDAA7A4F4C3BFC6` (break `/Game/Blueprint/Unit/Utils/FUnits` (`BlueprintMapLibrary.Map_Find` _unitsfromteam _team))))
        (`KismetArrayLibrary.Array_Append` (`local.tempUnitArray`) (`|MakeArray` _hostedunit))
        (`BlueprintMapLibrary.Map_Add` _unitsfromteam _team (make `/Game/Blueprint/Unit/Utils/FUnits` (`local.tempUnitArray`)))
        (add `/Game/Blueprint/Unit/BP_Unit.Dispatch_OnDeath` _hostedunit (`|CreateDelegate` :!event `OnUnitDeath`))))))

(fn `GetClosestEnemyUnit`
  (params (InUnit :type "/Game/Blueprint/Unit/BP_Unit Object Reference"))
  (returns (ReturnValue :type "/Game/Blueprint/Unit/BP_Unit Object Reference"))
  (locals (closestDistance :type "Float (double-precision)" :default 20000000.0) (team :type Integer :default 0) (tempClosestUnit :type "/Game/Blueprint/Unit/BP_Unit Object Reference"))
  (set `local.team` (`/Game/Blueprint/Unit/BP_Unit.Team` InUnit))
  (for _array_element (`self.Units`)
    (if (`|EnumInequality` (`/Game/Blueprint/Unit/BP_Unit.AIState` _array_element) "NewEnumerator3")
      (if (!= (`/Game/Blueprint/Unit/BP_Unit.Team` _array_element) (`local.team`))
        (bind _returnvalue (`self.GetDistanceTo` _array_element (`local.InUnit`)))
        (if (<= _returnvalue (`local.closestDistance`))
          (set `local.closestDistance` _returnvalue)
          (set `local.tempClosestUnit` _array_element)))))
  (return (`local.tempClosestUnit`)))

(fn `IsAreaEmpty`
  (params (Squares :type "Array of /Game/Blueprint/Level/BP_Square Object Reference") (GridX :type "Float (double-precision)") (GridY :type "Float (double-precision)") (BattleFieldX :type "Float (double-precision)") (BattleFieldY :type "Float (double-precision)") (FirstSquareTransform :type "Transform Structure") (SquareWidth :type "Float (double-precision)") (Team :type Byte) (TowerDistanceFromBorder :type Integer))
  (returns (IsAreaEmpty :type Boolean))
  (bind _output_get (set `self.SpaceToYBorder` (`KismetMathLibrary.FTrunc` (/ (- (`local.BattleFieldX`) (`local.GridX`)) 2.0))))
  (set `self.SquareID` (* _output_get (`KismetMathLibrary.FTrunc` (`local.BattleFieldX`))))
  (switch `int` (`KismetMathLibrary.Conv_ByteToInt` (`local.Team`))
    (:`0`
      (set `self.YSpaceBelowArea` (`local.TowerDistanceFromBorder`))
      (set `self.YSpaceAboveArea` (- (- (`KismetMathLibrary.FTrunc` (`local.BattleFieldY`)) (`self.YSpaceBelowArea`)) (`KismetMathLibrary.FTrunc` (`local.GridY`)))))
    (:`1`
      (set `self.YSpaceBelowArea` (+ (`KismetMathLibrary.FTrunc` (`local.BattleFieldY`)) (`local.TowerDistanceFromBorder`)))
      (set `self.YSpaceAboveArea` (`local.TowerDistanceFromBorder`))))
  (for _ (range (+ (`KismetMathLibrary.FTrunc` (- (`local.GridX`) 1.0)) 1))
    (set `self.SquareID` (+ (`self.SquareID`) (`self.YSpaceBelowArea`)))
    (for _ (range (+ (`KismetMathLibrary.FTrunc` (- (`local.GridY`) 1.0)) 1))
      (`/Engine/EditorBlueprintResources/StandardMacros.IsValid` (`/Game/Blueprint/Level/BP_Square.HostedUnit` (`|GetArrayItem` (`local.Squares`) (`self.SquareID`)))
        (:`Is Valid`
          (return false))
        (:`Is Not Valid`
          (bind _result (`/Engine/EditorBlueprintResources/StandardMacros.IncrementInt` (`self.SquareID`))
            (:`  `
              (set `self.SquareID` _result))))))
    (set `self.SquareID` (+ (`self.SquareID`) (`self.YSpaceAboveArea`))))
  (return true))

(fn `OnUnitDeath`
  (params (InUnit :type "/Game/Blueprint/Unit/BP_Unit Object Reference"))
  (`self.RemoveUnitFromTeam` InUnit))

(fn `RemoveUnitFromTeam`
  (params (InUnit :type "/Game/Blueprint/Unit/BP_Unit Object Reference"))
  (locals (tempUnits :type "Array of /Game/Blueprint/Unit/BP_Unit Object Reference"))
  (bind (_value _returnvalue) (`BlueprintMapLibrary.Map_Find` (`self.UnitsFromTeam`) (`/Game/Blueprint/Unit/BP_Unit.Team` InUnit)))
  (if _returnvalue
    (bind _output_get (set `local.tempUnits` (`.Units_3_D36FB76C40AE2CBD0FDAA7A4F4C3BFC6` (break `/Game/Blueprint/Unit/Utils/FUnits` _value))))
    (if (`KismetArrayLibrary.Array_Contains` _output_get InUnit)
      (`KismetArrayLibrary.Array_RemoveItem` (`local.tempUnits`) InUnit)
      (`BlueprintMapLibrary.Map_Add` (`self.UnitsFromTeam`) (`/Game/Blueprint/Unit/BP_Unit.Team` InUnit) (make `/Game/Blueprint/Unit/Utils/FUnits` (`local.tempUnits`))))))

(fn `SpawnUnits`
  (params (GridX :type "Float (double-precision)") (GridY :type "Float (double-precision)") (BattleFieldX :type "Float (double-precision)") (BattleFieldY :type "Float (double-precision)") (FirstSquareTransform :type "Transform Structure") (SquareWidth :type "Float (double-precision)") (UnitsToSpawn :type "Map of Integer to /Game/Blueprint/Unit/BP_Unit Object Reference") (Team :type Byte) (IsAreaEmpty :type Boolean) (TowerDistanceFromBorder :type "Float (double-precision)"))
  (locals (CurrentTransform :type "Transform Structure" :default "3800.000000,-5550.000000,195.000000|0.000000,0.000000,0.000000|1.000000,1.000000,1.000000") (LoopCount :type Integer) (StartXLocation :type "Float (double-precision)" :default 0.0) (StartYLocation :type "Float (double-precision)" :default 0.0) (Rotation :type "Rotator Structure" :default (struct)) (NewLocalVar_0 :type "Float (double-precision)"))
  (bind _startylocation (`local.StartYLocation`))
  (bind (_value _returnvalue) (`BlueprintMapLibrary.Map_Find` (`local.UnitsToSpawn`) (`local.LoopCount`)))
  (bind _returnvalue_2 (* (`local.TowerDistanceFromBorder`) (`local.SquareWidth`)))
  (switch `int` (`KismetMathLibrary.Conv_ByteToInt` Team)
    (:`0`
      (set `local.Rotation` (struct))
      (set `local.StartYLocation` (.y (.location FirstSquareTransform))))
    (:`1`
      (set `local.Rotation` (struct :`Yaw` 180.0))
      (set `local.StartYLocation` (+ (.y (.location FirstSquareTransform)) (* (- (`local.BattleFieldY`) (`local.GridY`)) (`local.SquareWidth`))))))
  (bind _output_get (set `local.CurrentTransform` (`KismetMathLibrary.MakeTransform` (`KismetMathLibrary.MakeVector` (+ (.x (.location FirstSquareTransform)) (* (/ (- BattleFieldX GridX) 2.0) (`local.SquareWidth`))) (`local.StartYLocation`) (.z (.location FirstSquareTransform))) (`local.Rotation`) (.scale FirstSquareTransform))))
  (set `local.StartXLocation` (.x (.location _output_get)))
  (if (not (`local.IsAreaEmpty`))
    (switch `int` 0
      (:`0`
        (set `local.StartYLocation` (+ _startylocation _returnvalue_2)))
      (:`1`
        (set `local.StartYLocation` (- _startylocation _returnvalue_2)))))
  (for _ (range (+ (`KismetMathLibrary.FTrunc` (- (`local.GridX`) 1.0)) 1))
    (for _index (range (+ (`KismetMathLibrary.FTrunc` (- (`local.GridY`) 1.0)) 1))
      (if (not (== _index 0))
        (set `local.CurrentTransform` (`KismetMathLibrary.MakeTransform` (`KismetMathLibrary.MakeVector` (.x (.location (`local.CurrentTransform`))) (+ (.y (.location (`local.CurrentTransform`))) (`local.SquareWidth`)) (.z (.location (`local.CurrentTransform`)))) (.rotation (`local.CurrentTransform`)) (.scale (`local.CurrentTransform`)))))
      (if _returnvalue
        (`AIBlueprintHelperLibrary.SpawnAIFromClass` (`GameplayStatics.GetObjectClass` _value) "/Game/Blueprint/AI/BT_Unit.BT_Unit" (.location (`local.CurrentTransform`)) (.rotation (`local.CurrentTransform`)) false null)
        (`/Engine/EditorBlueprintResources/StandardMacros.IncrementInt` (`local.LoopCount`))))
    (set `local.CurrentTransform` (`KismetMathLibrary.MakeTransform` (`KismetMathLibrary.MakeVector` (+ (.x (.location (`local.CurrentTransform`))) (`local.SquareWidth`)) (`local.StartYLocation`) (.z (.location (`local.CurrentTransform`)))) (.rotation (`local.CurrentTransform`)) (.scale (`local.CurrentTransform`))))))

(fn `StartCombat`
  (`self.FindUnitsInBattlefield`)
  (`self.FindUnitsInGrid`)
  (`/Game/Blueprint/Unit/BP_Unit.StartCombat` (`self.Units`)))

(fn `UserConstructionScript`
  (`parent.UserConstructionScript`))