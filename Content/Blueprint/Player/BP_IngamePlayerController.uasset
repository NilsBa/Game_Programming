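; In-game player controller for a two-team, square-based unit game, assigning the team by server or client and handling pause, end screens and alert sounds.
; Each tick a cursor sphere trace finds the focused square, highlights its unit and interpolates any carried unit.
; Own units outside the battlefield move by click or timer-detected drag, swapping with occupants.
; Unit and tower spawns, final moves and square assignments go through BP_IngameMode.
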(event `EndScreen`
  (params (LoseTeam :type Integer) (NewParam :type "PlayerController Object Reference"))
  (`WidgetLayoutLibrary.RemoveAllWidgets`)
  (if (== LoseTeam (`self.Team`))
    (bind _returnvalue (`|CreateWidget` "/Game/OwnContent/Blueprints/LoseScreen.LoseScreen_C" self))
    (switch `int` (`self.Team`)
      (:`0`
        (set `/Game/OwnContent/Blueprints/LoseScreen.enemyDeaths` (`self.Player2Deaths`) _returnvalue)
        (set `/Game/OwnContent/Blueprints/LoseScreen.ownDeaths` (`self.Player1Deaths`) _returnvalue))
      (:`1`
        (set `/Game/OwnContent/Blueprints/LoseScreen.enemyDeaths` (`self.Player1Deaths`) _returnvalue)
        (set `/Game/OwnContent/Blueprints/LoseScreen.ownDeaths` (`self.Player2Deaths`) _returnvalue)))
    (`UserWidget.AddToViewport` _returnvalue 0)
    (else
      (bind _returnvalue_2 (`|CreateWidget` "/Game/OwnContent/Blueprints/WinScreen.WinScreen_C" self))
      (switch `int` (`self.Team`)
        (:`0`
          (set `/Game/OwnContent/Blueprints/WinScreen.enemyDeaths` 0 _returnvalue_2)
          (set `/Game/OwnContent/Blueprints/WinScreen.ownDeaths` (`self.Player1Deaths`) _returnvalue_2))
        (:`1`
          (set `/Game/OwnContent/Blueprints/WinScreen.enemyDeaths` (`self.Player1Deaths`) _returnvalue_2)
          (set `/Game/OwnContent/Blueprints/WinScreen.ownDeaths` (`self.Player2Deaths`) _returnvalue_2)))
      (`UserWidget.AddToViewport` _returnvalue_2 0))))

(event `self.ReceiveBeginPlay`
  ;[1 1 1] Clear Loading Screen
  (`|ExecutionSequence`
    (:`then_0`
      (`KismetSystemLibrary.Delay` 0.1)
      (`WidgetBlueprintLibrary.SetInputMode_GameAndUIEx` self null "DoNotLock" false)
      (if (`self.IsLocalController`)
        (`WidgetLayoutLibrary.RemoveAllWidgets`)))
    (:`then_1`
      ;[1 1 1] SetTeam
      (if (`KismetSystemLibrary.IsServer`)
        (set `self.Team` 0)
        (else
          (set `self.Team` 1))))))

(event `Key|Escape` :paused true
  (params (Key :type "Key Structure"))
  (bind _pausemenuref (`self.PauseMenuRef`))
  ;[1 1 1] Pause/unpause game
  (:`Pressed`
    (`/Engine/EditorBlueprintResources/StandardMacros.IsValid` (`self.PauseMenuRef`) :!label _label
      (:`Is Valid`
        _)
      (:`Is Not Valid`
        (bind _returnvalue (`|CreateWidget` "/Game/Blueprint/Player/Widgets/WGT_PauseMenu.WGT_PauseMenu_C"))
        (bind _output_get (set `self.PauseMenuRef` _returnvalue))))
    (if (`self.bIsPaused`)
      (if (`Widget.IsVisible` _output_get)
        (`Widget.RemoveFromParent` _output_get)
        (set `self.bIsPaused` false)
        (set `self.bShowMouseCursor` true)
        (`WidgetBlueprintLibrary.SetInputMode_GameOnly` null)
        (else
          (bind _foundwidgets (`WidgetBlueprintLibrary.GetAllWidgetsOfClass` "/Game/MainMenu/W_VideoSettings.W_VideoSettings_C"))
          (for _array_element _foundwidgets
            (`Widget.RemoveFromParent` _array_element))
          (bind _foundwidgets_2 (`WidgetBlueprintLibrary.GetAllWidgetsOfClass` "/Game/MainMenu/W_AudioSettings.W_AudioSettings_C"))
          (for _array_element_2 _foundwidgets_2
            (`Widget.RemoveFromParent` _array_element_2))
          (`/Engine/EditorBlueprintResources/StandardMacros.IsValid` _pausemenuref
            (:`Is Valid`
              (`UserWidget.AddToViewport` _pausemenuref 0)
              (`Widget.SetVisibility` _pausemenuref "Visible"))
            (:`Is Not Valid`
              (bind _returnvalue_2 (`|CreateWidget` "/Game/Blueprint/Player/Widgets/WGT_PauseMenu.WGT_PauseMenu_C"))
              (bind _output_get_2 (set `self.PauseMenuRef` _returnvalue_2))
              (`UserWidget.AddToViewport` _output_get_2 0)))))
      (else
        (`UserWidget.AddToViewport` _output_get 0)
        (set `self.bIsPaused` true)
        (set `self.bShowMouseCursor` true)
        (`WidgetBlueprintLibrary.SetInputMode_UIOnlyEx` null _output_get "LockInFullscreen")))))

(event `Key|P`
  (params (Key :type "Key Structure"))
  ;[1 1 1] Pause/unpause game
  (:`Pressed`
    (goto _label)))

(event `self.ReceiveTick`
  (params (DeltaSeconds :type "Float (single-precision)"))
  (`parent.ReceiveTick` DeltaSeconds)
  (`self.FindFocusedSquare`)
  (`self.UpdateMovedUnitLocation`))

(event `Key|LeftMouseButton`
  (params (Key :type "Key Structure"))
  (:`Pressed`
    (`self.DragUnit`))
  (:`Released`
    (`self.DropUnit`)))

(event `FinalStopMove`
  (bind _rootcomponent (`Actor.RootComponent` (`self.MovingUnit`)))
  (bind _returnvalue (+ (`self.K2_GetActorLocation` (`self.LastFocusedSquare`)) (0.0 0.0 50.0)))
  (bind _returnvalue_2 (`KismetMathLibrary.MakeRotator` (.roll (`KismetMathLibrary.FindLookAtRotation` _returnvalue (`KismetMathLibrary.Conv_IntVectorToVector` (`GameplayStatics.GetWorldOriginLocation`)))) (.pitch (`KismetMathLibrary.FindLookAtRotation` _returnvalue (`KismetMathLibrary.Conv_IntVectorToVector` (`GameplayStatics.GetWorldOriginLocation`)))) (- (.yaw (`KismetMathLibrary.FindLookAtRotation` _returnvalue (`KismetMathLibrary.Conv_IntVectorToVector` (`GameplayStatics.GetWorldOriginLocation`)))) 90.0)))
  (bind _returnvalue_3 (`GameplayStatics.GetCurrentLevelName` true))
  (`|ExecutionSequence`
    (:`then_0`
      (if (`KismetStringLibrary.EqualEqual_StrStr` _returnvalue_3 "Map1")
        (cast `/Game/Blueprint/Player/BP_IngamePlayerController` (`GameplayStatics.GetPlayerController` 0))
        (`self.MoveComponent` _rootcomponent _returnvalue _returnvalue_2)
        (else
          (bind _asbp_ingame_player_controller (cast `/Game/Blueprint/Player/BP_IngamePlayerController` (`GameplayStatics.GetPlayerController` 0)))
          (`self.MoveComponent` _asbp_ingame_player_controller _rootcomponent (+ _returnvalue (0.0 0.0 100.0)) _returnvalue_2))))
    (:`then_1`
      (`/Engine/EditorBlueprintResources/StandardMacros.IsValid` (`self.GetFocusedSquare`)
        (:`Is Valid`
          _)
        (:`Is Not Valid`
          (`/Game/Blueprint/Unit/BP_Unit.SetFocused` (`self.MovingUnit`) false)))
      (set `self.MovingUnit` null)
      (set `self.bMovingUnit` false))))

(event `MoveComponent`
  (params (Component :type "SceneComponent Object Reference") (TargetLocation :type "Vector Structure") (TargetRotation :type "Rotator Structure"))
  (bind _asbp_ingame_mode (cast `/Game/Blueprint/GameSystem/BP_IngameMode` (`GameplayStatics.GetGameMode`)))
  (bind _output_get (set `self.GameMode` _asbp_ingame_mode))
  (`/Game/Blueprint/GameSystem/BP_IngameMode.MoveComponentTo` _output_get Component TargetLocation TargetRotation))

(event `SpawnUnitOnServer`
  (params (SpawnTransform :type "Transform Structure") (UnitRow :type "DataTableRowHandle Structure") (OwningPlayer :type "PlayerController Object Reference"))
  (bind _asbp_ingame_mode (cast `/Game/Blueprint/GameSystem/BP_IngameMode` (`GameplayStatics.GetGameMode`)))
  (`/Game/Blueprint/GameSystem/BP_IngameMode.SpawnUnit` _asbp_ingame_mode SpawnTransform UnitRow)
  (bind _asbp_ingame_player_controller (cast `/Game/Blueprint/Player/BP_IngamePlayerController` OwningPlayer))
  (`self.SetDraggingUnit` _asbp_ingame_player_controller))

(event `SetDraggingUnit`
  (`self.DragUnit`))

(event `PlayLowHealthSound`
  (if (not (`self.bIsLowHealthSoundPlaying`))
    (set `self.bIsLowHealthSoundPlaying` true)
    (bind _output_get (set `self.LowHealthSound` "/Game/BackgroundSound/BaseSounds/LowHealth.LowHealth"))
    (`GameplayStatics.PlaySound2D` _output_get 0.8 1.0 0.0 null null)
    (`KismetSystemLibrary.Delay` (+ (`SoundBase.Duration` _output_get) 1.0))
    (set `self.bIsLowHealthSoundPlaying` false)))

(event `SetHostedUnitTarget`
  (params (BPUnit :type "/Game/Blueprint/Unit/BP_Unit Object Reference") (Square :type "/Game/Blueprint/Level/BP_Square Object Reference"))
  (bind _asbp_ingame_player_controller (cast `/Game/Blueprint/Player/BP_IngamePlayerController` (`GameplayStatics.GetPlayerController` 0)))
  (`self.SetHostedUnitTargetOnServer` _asbp_ingame_player_controller BPUnit Square))

(event `SetHostedUnitTargetOnServer`
  (params (BPUnit :type "/Game/Blueprint/Unit/BP_Unit Object Reference") (Square :type "/Game/Blueprint/Level/BP_Square Object Reference"))
  (bind _asbp_ingame_mode (cast `/Game/Blueprint/GameSystem/BP_IngameMode` (`GameplayStatics.GetGameMode`)))
  (`/Game/Blueprint/GameSystem/BP_IngameMode.SetHostedUnitTarget` _asbp_ingame_mode BPUnit Square))

(event `PlayDamageSound`
  (if (not (`self.bIsDamageSoundPlaying`))
    (set `self.bIsDamageSoundPlaying` true)
    (bind _output_get (set `self.DamageSound` "/Game/BackgroundSound/BaseSounds/UnderAttack.UnderAttack"))
    (`GameplayStatics.PlaySound2D` _output_get 0.4 1.0 0.0 null null)
    (`KismetSystemLibrary.Delay` (+ (`SoundBase.Duration` _output_get) 5.0))
    (set `self.bIsDamageSoundPlaying` false)))

(event `SpawnTowerOnServer`
  (params (TowerPosition :type Integer) (TowerClass :type Integer))
  (bind _asbp_ingame_mode (cast `/Game/Blueprint/GameSystem/BP_IngameMode` (`GameplayStatics.GetGameMode`)))
  (`/Game/Blueprint/GameSystem/BP_IngameMode.SpawnTowersOnSquare` _asbp_ingame_mode TowerPosition TowerClass))

(fn `AddUnitDeath`
  (params (player :type Integer))
  (returns (Deaths :type Integer))
  (switch `int` player
    (:`0`
      (bind _output_get (set `self.Player1Deaths` (+ (`self.Player1Deaths`) 1)))
      (`KismetSystemLibrary.PrintString` "Own Unit was killed ")
      (return _output_get))
    (:`1`
      (bind _output_get_2 (set `self.Player2Deaths` (+ (`self.Player2Deaths`) 1)))
      (`KismetSystemLibrary.PrintString` "Own Unit was killed ")
      (return _output_get_2))))

(fn `DragUnit`
  (bind _returnvalue (`self.GetUnitInSquare`))
  (bind _returnvalue_2 (`self.GetFocusedSquare`))
  (if (`KismetSystemLibrary.IsValid` _returnvalue)
    (if (== (`self.Team`) (`/Game/Blueprint/Unit/BP_Unit.Team` _returnvalue))
      (if (not (`self.bMovingUnit`))
        (`/Engine/EditorBlueprintResources/StandardMacros.IsValid` _returnvalue_2
          (:`Is Valid`
            (if (not (`/Game/Blueprint/Level/BP_Square.bIsInBattlefield` _returnvalue_2))
              (if (`/Game/Blueprint/Level/BP_Square.bIsTowerSquare` _returnvalue_2)
                (if (`/Game/Blueprint/Unit/BP_Unit.bHasPriority` (`self.GetUnitInSquare`))
                  (`self.HasUnitToFocus` :!label _label
                    (:`Valid`
                      (`self.StartMovingUnit`)
                      (bind _returnvalue_3 (`KismetSystemLibrary.K2_SetTimerDelegate` (`|CreateDelegate` :!event `StartDragging`) (`self.DragTriggerDelay`)))
                      (set `self.DraggingTimer` _returnvalue_3))))
                (else
                  (goto _label))))))
        (elif (not (`self.bDragging`))
          (`self.StopMovingUnit`))))))

(fn `DropUnit`
  (if (`self.bDragging`)
    (`self.StopDragging`)
    (else
      (`KismetSystemLibrary.K2_ClearAndInvalidateTimerHandle` (`self.DraggingTimer`)))))

(fn `FindFocusedSquare`
  (bind _output_get (set `self.CursorLocation` (`.Location` (`GameplayStatics.BreakHitResult` (`self.GetHitResultUnderCursorByChannel` "TraceTypeQuery3")))))
  (bind _outhits (`KismetSystemLibrary.SphereTraceMulti` :`Start` _output_get :`End` (+ _output_get (0.0 0.0 1.0)) :`Radius` 5.0 :`TraceChannel` "TraceTypeQuery4" :`DrawTime` 1.0))
  (if (> (`KismetArrayLibrary.Array_Length` _outhits) 0)
    (bind (_bblockinghit _binitialoverlap _time _distance _location _impactpoint _normal _impactnormal _physmat _hitactor) (`GameplayStatics.BreakHitResult` (`|GetArrayItem` _outhits)))
    (`/Engine/EditorBlueprintResources/StandardMacros.IsValid` _hitactor
      (:`Is Valid`
        (bind _asbp_square (cast `/Game/Blueprint/Level/BP_Square` _hitactor)
          (:`then`
            (if (!= _asbp_square (`self.FocusedSquare`))
              (`self.UnfocusSquare`)
              (`self.SetFocusedSquare` _asbp_square)))
          (:`CastFailed`
            (`self.UnfocusSquare` :!label _label))))
      (:`Is Not Valid`
        (goto _label)))))

(fn `GetFocusedSquare`
  (returns (ReturnValue :type "/Game/Blueprint/Level/BP_Square Object Reference"))
  (return (`self.FocusedSquare`)))

(fn `GetMovingUnit`
  (returns (ReturnValue :type "/Game/Blueprint/Unit/BP_Unit Object Reference"))
  (return (`self.MovingUnit`)))

(fn `GetUnitInSquare`
  (returns (ReturnValue :type "/Game/Blueprint/Unit/BP_Unit Object Reference"))
  (return (`/Game/Blueprint/Level/BP_Square.HostedUnit` (`self.GetFocusedSquare`))))

(fn `SetFocusedSquare`
  (params (Square :type "/Game/Blueprint/Level/BP_Square Object Reference"))
  (set `self.FocusedSquare` Square)
  (if (not (`self.bMovingUnit`))
    (`self.HasUnitToFocus`
      (:`Valid`
        (`/Game/Blueprint/Unit/BP_Unit.SetFocused` (`self.GetUnitInSquare`) true)))))

(fn `StartDragging`
  (set `self.bDragging` true))

(fn `StartMovingUnit`
  (bind _returnvalue (`self.GetFocusedSquare`))
  (set `self.MovingUnit` (`self.GetUnitInSquare`))
  (set `self.bMovingUnit` true)
  (`/Game/Blueprint/Unit/BP_Unit.SetDragState` (`self.GetMovingUnit`) true)
  (set `self.InitialSquare` _returnvalue)
  (`self.SetHostedUnitTarget` null _returnvalue)
  (set `/Game/Blueprint/Level/BP_Square.HostedUnit` null _returnvalue))

(fn `StopDragging`
  (`self.StopMovingUnit`)
  (set `self.bDragging` false))

(fn `StopMovingUnit`
  (bind _returnvalue (`self.GetFocusedSquare`))
  (bind _returnvalue_2 (`self.GetMovingUnit`))
  (bind _lastfocusedsquare (`self.LastFocusedSquare`))
  (`/Engine/EditorBlueprintResources/StandardMacros.IsValid` _returnvalue
    (:`Is Valid`
      (set `self.LastFocusedSquare` _returnvalue)
      (`self.HasUnitToFocus`
        (:`Valid`
          (`self.SwapUnitPositions` (`self.GetUnitInSquare`) (`self.InitialSquare`)))
        (:`Invalid`
          _))
      (`/Game/Blueprint/Unit/BP_Unit.SetDragState` (`self.GetMovingUnit`) false)
      (`self.SetHostedUnitTarget` _returnvalue_2 _lastfocusedsquare)
      (set `/Game/Blueprint/Level/BP_Square.HostedUnit` _returnvalue_2 _lastfocusedsquare)
      (`self.FinalStopMove`))))

(fn `SwapUnitPositions`
  (params (ForUnit :type "/Game/Blueprint/Unit/BP_Unit Object Reference") (InSquare :type "/Game/Blueprint/Level/BP_Square Object Reference"))
  (`self.K2_SetActorLocation` ForUnit (+ (`self.K2_GetActorLocation` InSquare) (0.0 0.0 50.0)) false true)
  (`self.SetHostedUnitTarget` ForUnit InSquare)
  (set `/Game/Blueprint/Level/BP_Square.HostedUnit` ForUnit InSquare))

(fn `UnfocusSquare`
  (bind _focusedsquare (`self.FocusedSquare`))
  (`/Engine/EditorBlueprintResources/StandardMacros.IsValid` (`self.GetFocusedSquare`)
    (:`Is Valid`
      (if (not (`self.bMovingUnit`))
        (`self.HasUnitToFocus`
          (:`Valid`
            (`/Game/Blueprint/Unit/BP_Unit.SetFocused` (`self.GetUnitInSquare`) false))
          (:`Invalid`
            _))))
    (:`Is Not Valid`
      _))
  (`/Engine/EditorBlueprintResources/StandardMacros.IsValid` _focusedsquare
    (:`Is Valid`
      (set `self.LastFocusedSquare` _focusedsquare))
    (:`Is Not Valid`
      _))
  (set `self.FocusedSquare` null))

(fn `UpdateMovedUnitLocation`
  (locals (squareTempLoc :type "Vector Structure" :default (0.0 0.0 0.0)))
  (bind _returnvalue (`self.GetMovingUnit`))
  (bind _returnvalue_2 (`self.GetFocusedSquare`))
  (bind _cursorlocation (`self.CursorLocation`))
  (bind _returnvalue_3 (`self.K2_GetActorLocation` _returnvalue))
  (`/Engine/EditorBlueprintResources/StandardMacros.IsValid` _returnvalue_2
    (:`Is Valid`
      (set `local.squareTempLoc` (`self.K2_GetActorLocation` _returnvalue_2)))
    (:`Is Not Valid`
      (set `local.squareTempLoc` _cursorlocation)))
  (if (`self.bMovingUnit`)
    (`self.K2_SetActorLocation` _returnvalue (`KismetMathLibrary.VInterpTo` _returnvalue_3 (`KismetMathLibrary.MakeVector` (.x (select `bool` (`self.bSnapMove`) :`false` _cursorlocation :`true` (`local.squareTempLoc`))) (.y (select `bool` (`self.bSnapMove`) :`false` _cursorlocation :`true` (`local.squareTempLoc`))) (.z _returnvalue_3)) (`GameplayStatics.GetWorldDeltaSeconds`) (`self.MoveSpeed`)) false false)))

(fn `UserConstructionScript`
  (`parent.UserConstructionScript`))